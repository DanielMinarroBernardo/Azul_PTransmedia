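; BP_Hilo is an actor that shows a Niagara thread effect associated with a spline route (Recorrido).
; On BeginPlay it sets the effect's SpawnRate to the spline's length, so particle emission scales with the route.
; Any overlap with its Box calls SetSpline, whose body is not shown here, then resets the Niagara system.
; Activate and Deactivate calls on the effect are left unconnected.
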(event `self.ReceiveBeginPlay`
  (`NiagaraComponent.SetVariableFloat` (`self.HiloNiagara`) "SpawnRate" (`SplineComponent.GetSplineLength` (`self.Recorrido`))))

(event `self.Box.OnComponentBeginOverlap`
  (params (OverlappedComponent :type "PrimitiveComponent Object Reference") (OtherActor :type "Actor Object Reference") (OtherComp :type "PrimitiveComponent Object Reference") (OtherBodyIndex :type Integer) (bFromSweep :type Boolean) (SweepResult :type "HitResult Structure (by ref)"))
  (`self.SetSpline`)
  (`NiagaraComponent.ResetSystem` (`self.HiloNiagara`)))

(fn `UserConstructionScript`)