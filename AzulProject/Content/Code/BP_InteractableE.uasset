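; BP_InteractableE is an interactable actor that prompts the player, in Spanish, to press E to pick up the object.
; BeginPlay sets the text on its WBP_InteractableE widget.
; Trigger overlaps show or hide that widget and register or clear the actor as BP_FirstPersonCharacter's InteractableObjet.
; InteractE is an empty event, and the animation and hand-socket attach nodes are unconnected, so no pickup happens here.
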(event `self.ReceiveBeginPlay`
  (bind _aswbp_interactable_e (cast `/Game/UI/WBP_InteractableE` (`WidgetComponent.GetWidget` (`self.Widget`))))
  (set `/Game/UI/WBP_InteractableE.Texto` "Pulsa E para coger el \"objeto\"" _aswbp_interactable_e))

(event `self.Trigger.OnComponentBeginOverlap`
  (params (OverlappedComponent :type "PrimitiveComponent Object Reference") (OtherActor :type "Actor Object Reference") (OtherComp :type "PrimitiveComponent Object Reference") (OtherBodyIndex :type Integer) (bFromSweep :type Boolean) (SweepResult :type "HitResult Structure (by ref)"))
  (bind _asbp_first_person_character (cast `/Game/FirstPerson/Blueprints/BP_FirstPersonCharacter` OtherActor))
  (bind _output_get (set `self.As BP First Person Character` _asbp_first_person_character))
  (set `/Game/FirstPerson/Blueprints/BP_FirstPersonCharacter.InteractableObjet` self _output_get)
  (`SceneComponent.SetVisibility` (`self.Widget`) true false))

(event `self.Trigger.OnComponentEndOverlap`
  (params (OverlappedComponent :type "PrimitiveComponent Object Reference") (OtherActor :type "Actor Object Reference") (OtherComp :type "PrimitiveComponent Object Reference") (OtherBodyIndex :type Integer))
  (bind _asbp_first_person_character (cast `/Game/FirstPerson/Blueprints/BP_FirstPersonCharacter` OtherActor))
  (set `/Game/FirstPerson/Blueprints/BP_FirstPersonCharacter.InteractableObjet` null _asbp_first_person_character)
  (`SceneComponent.SetVisibility` (`self.Widget`) false false))

(event `self.InteractE`)

(fn `UserConstructionScript`)